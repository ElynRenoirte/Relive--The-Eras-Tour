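; Player controller that shows the mouse cursor in Game and UI input mode and lets mouse dragging rotate an outfit character.
; While IsDragging is set, Tick passes horizontal mouse delta to the OutfitCharacter's rotate function and prints a debug string; neither variable is set here.
; The virtual cursor input events and RotateOutfitCharacter function are empty, with leftover cursor-movement and direct-rotation nodes disconnected.
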(event `self.ReceiveBeginPlay`
  (set `self.bShowMouseCursor` true)
  (set `self.bEnableClickEvents` true)
  (set `self.bEnableMouseOverEvents` true)
  (`WidgetBlueprintLibrary.SetInputMode_GameAndUIEx` (`GameplayStatics.GetPlayerController` 0) null "LockOnCapture" false))

(event `EnhancedInput|/Game/InpuAction_CursorMove`
  (params (ActionValue :type "Vector2D Structure") (ElapsedSeconds :type "Float (double-precision)") (TriggeredSeconds :type "Float (double-precision)") (InputAction :type "InputAction Object Reference" :default "/Game/InpuAction_CursorMove.InpuAction_CursorMove")))

(event `EnhancedInput|/Game/InputAction_VirtualClick`
  (params (ActionValue :type Boolean) (ElapsedSeconds :type "Float (double-precision)") (TriggeredSeconds :type "Float (double-precision)") (InputAction :type "InputAction Object Reference" :default "/Game/InputAction_VirtualClick.InputAction_VirtualClick")))

(event `self.ReceiveTick`
  (params (DeltaSeconds :type "Float (single-precision)"))
  (if (`self.IsDragging`)
    (`KismetSystemLibrary.PrintString` "is dragging")
    (`/Engine/EditorBlueprintResources/StandardMacros.IsValid` (`self.OutfitCharacter`)
      (:`Is Valid`
        (`/Game/character_3rdperson/character_only_pose_as_rest_pose_Blueprint.RotateCharacterFunction` (`self.OutfitCharacter`) (`self.GetInputMouseDelta`))))))

(fn `RotateOutfitCharacter (float DeltaX)`)

(fn `UserConstructionScript`)