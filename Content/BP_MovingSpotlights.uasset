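; Spotlight actor that plays a timed light show from BeginPlay, like choreographed stage lighting.
; A timeline sweeps yaw between min and max rotation for a set number of loops, alongside optional fade-out and flash branches.
; The flash branch chains timelines and hard-coded delays to tilt the light up, down and up again.
; A delayed, optional timeline steps through six preset colors; the timer-based color change is unused.
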(event `self.ReceiveBeginPlay`
  (`|ExecutionSequence`
    (:`then_0`
      (bind (_direction _rotationtrack) (`Timeline|Timeline_MovingLights` :!label _label)
        (:`Update`
          (`SceneComponent.K2_SetRelativeRotation` (`self.SpotLight`) (`KismetMathLibrary.MakeRotator` 0.0 0.0 (`KismetMathLibrary.Lerp` (`self.MinRotation`) (`self.MaxRotation`) _rotationtrack)) false false))
        (:`Finished`
          (`/Engine/EditorBlueprintResources/StandardMacros.IncrementInt` (`self.LoopCount`)
            (:`  `
              (if (< (`self.LoopCount`) (`self.MaxLoops`))
                (goto _label :!via `PlayFromStart`)))))))
    (:`then_1`
      (`KismetSystemLibrary.Delay` 0.1)
      (if (`self.ShouldFadeOut`)
        (bind (_direction_2 _fadetrack) (`Timeline|LightsFadeOut`)
          (:`Update`
            (`LightComponent.SetIntensity` (`self.SpotLight`) _fadetrack)))))
    (:`then_2`
      (if (`self.ShouldFlash`)
        (`LightComponent.SetIntensity` (`self.SpotLight`) 0.0)
        (`KismetSystemLibrary.Delay` 17.29)
        (bind (_direction_3 _flashtrack) (`Timeline|TL_FlashLights`)
          (:`Update`
            (`LightComponent.SetIntensity` (`self.SpotLight`) _flashtrack))
          (:`Finished`
            (`KismetSystemLibrary.Delay` 8.91)
            (`LightComponent.SetIntensity` (`self.SpotLight`) 160.0)
            (bind (_direction_4 _upwardrotationalpha) (`Timeline|TL_UpwardRotation`)
              (:`Update`
                (`SceneComponent.K2_SetRelativeRotation` (`self.SpotLight`) (`KismetMathLibrary.RLerp` (`self.DownRotation`) (`self.UpRotation`) _upwardrotationalpha) false false))
              (:`Finished`
                (`KismetSystemLibrary.Delay` (`self.DownDelay`))
                (bind (_direction_5 _lights_down_alpha) (`Timeline|TL_LightsDown`)
                  (:`Update`
                    (`SceneComponent.K2_SetRelativeRotation` (`self.SpotLight`) (`KismetMathLibrary.RLerp` (`self.UpRotation`) (`self.DownRotation`) _lights_down_alpha) false false))
                  (:`Finished`
                    (`KismetSystemLibrary.Delay` 43.0)
                    (bind (_direction_6 _upwardrotationalpha_2) (`Timeline|Timeline`)
                      (:`Update`
                        (`SceneComponent.K2_SetRelativeRotation` (`self.SpotLight`) (`KismetMathLibrary.RLerp` (`self.DownRotation`) (`self.UpRotation`) _upwardrotationalpha_2) false false)))))))))))
    (:`then_3`
      (`KismetSystemLibrary.Delay` 33.0)
      (if (`self.StayOn`)
        (bind (_direction_7 _colorindex) (`Timeline|ColorSequence`)
          (:`Update`
            (switch `int` (`KismetMathLibrary.FFloor` _colorindex)
              (:`0`
                (`LightComponent.SetLightColor` (`self.SpotLight`) (struct :`R` 0.514918 :`G` 0.38643 :`B` 0.552012 :`A` 1.0) true)
                (set `self.CurrentColorIndex` 1))
              (:`1`
                (`LightComponent.SetLightColor` (`self.SpotLight`) (struct :`R` 0.806952 :`G` 0.552012 :`B` 0.278894 :`A` 1.0) true)
                (set `self.CurrentColorIndex` 2))
              (:`2`
                (`LightComponent.SetLightColor` (`self.SpotLight`) (struct :`R` 0.822786 :`G` 0.456411 :`B` 0.603828 :`A` 1.0) true)
                (set `self.CurrentColorIndex` 3))
              (:`3`
                (`LightComponent.SetLightColor` (`self.SpotLight`) (struct :`R` 0.152926 :`G` 0.074214 :`B` 0.061246 :`A` 1.0) true)
                (set `self.CurrentColorIndex` 4))
              (:`4`
                (`LightComponent.SetLightColor` (`self.SpotLight`) (struct :`R` 0.508881 :`G` 0.623961 :`B` 0.473532 :`A` 1.0) true)
                (set `self.CurrentColorIndex` 5))
              (:`5`
                (`LightComponent.SetLightColor` (`self.SpotLight`) (struct :`R` 0.53948 :`G` 0.760525 :`B` 0.904661 :`A` 1.0) true)
                (set `self.CurrentColorIndex` 0)))))))))

(event `ChangeColor`)

(fn `UserConstructionScript`)