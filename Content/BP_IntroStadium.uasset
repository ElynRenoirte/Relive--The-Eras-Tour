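; Stadium intro actor that moves two fog banks and animates their density when play begins.
; BeginPlay assigns the first two StadiumFog-tagged BP_FogBankVolume actors as left and right, storing their start locations.
; TL_PartFog lerps both positions and sets both densities, though both banks target FogLeftEndLocation.
; SnapCameraToPlayer only casts the player character to BP_StadiumPlayer; its camera transform node is unconnected.
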(event `self.ReceiveBeginPlay`
  (bind _outactors (`GameplayStatics.GetAllActorsWithTag` "StadiumFog"))
  (`|ExecutionSequence`
    (:`then_0`
      (bind _asbp_fog_bank_volume (cast `/Game/NiagaraExamples/FX_Fog/BP_FogBankVolume` (`|GetArrayItem` _outactors)))
      (set `self.FogLeft` _asbp_fog_bank_volume)
      (set `self.FogLeftStartLocation` (`self.K2_GetActorLocation` (`self.FogLeft`)))
      (bind (_direction _fogalpha _fogdensity) (`Timeline|TL_PartFog` :!label _label)
        (:`Update`
          (`|ExecutionSequence`
            (:`then_0`
              (`self.K2_SetActorLocation` (`self.FogLeft`) (`KismetMathLibrary.VLerp` (`self.FogLeftStartLocation`) (`self.FogLeftEndLocation`) _fogalpha) false false))
            (:`then_1`
              (`self.K2_SetActorLocation` (`self.FogRight`) (`KismetMathLibrary.VLerp` (`self.FogRightStartLocation`) (`self.FogLeftEndLocation`) _fogalpha) false false))
            (:`then_2`
              (`/Game/NiagaraExamples/FX_Fog/BP_FogBankVolume.SetFogDensity` (`self.FogLeft`) _fogdensity))
            (:`then_3`
              (`/Game/NiagaraExamples/FX_Fog/BP_FogBankVolume.SetFogDensity` (`self.FogRight`) _fogdensity))))))
    (:`then_1`
      (bind _asbp_fog_bank_volume_2 (cast `/Game/NiagaraExamples/FX_Fog/BP_FogBankVolume` (`|GetArrayItem` _outactors 1)))
      (set `self.FogRight` _asbp_fog_bank_volume_2)
      (set `self.FogRightStartLocation` (`self.K2_GetActorLocation` (`self.FogRight`)))
      (goto _label))))

(event `SnapCameraToPlayer`
  (cast `/Game/BP_StadiumPlayer` (`GameplayStatics.GetPlayerCharacter` 0)))

(fn `UserConstructionScript`)